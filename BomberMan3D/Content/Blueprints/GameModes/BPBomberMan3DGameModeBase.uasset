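; Game mode for a two-player 3D Bomberman game that switches between gameplay and the end-of-match win screen.
; BeginPlay caches the game state and adds the win screen and countdown timer widgets to the viewport.
; Every Tick polls the game state's Result: "None" keeps play running with game-only input, while any other value shows the win screen, enables UI input and cursor for both controllers, and pauses the game.
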(event `self.ReceiveBeginPlay`
  (bind _asbpbomber_man_3dgame_state_base (cast `/Game/Blueprints/GameModes/BPBomberMan3DGameStateBase` (`GameplayStatics.GetGameState`)))
  (set `self.GameStateV` _asbpbomber_man_3dgame_state_base)
  (`|ExecutionSequence`
    (:`then_0`
      (bind _returnvalue (`|CreateWidget` "/Game/Blueprints/UMG/BPWinScreen.BPWinScreen_C"))
      (bind _output_get (set `self.WinScreen` _returnvalue))
      (`UserWidget.AddToViewport` _output_get 0))
    (:`then_1`
      (bind _returnvalue_2 (`|CreateWidget` "/Game/Blueprints/UMG/BPCoundownTimer.BPCoundownTimer_C"))
      (`UserWidget.AddToViewport` _returnvalue_2 0))))

(event `self.ReceiveTick`
  (params (DeltaSeconds :type "Float (single-precision)"))
  (bind _returnvalue (`GameplayStatics.GetPlayerControllerFromID` 0))
  (bind _returnvalue_2 (`GameplayStatics.GetPlayerControllerFromID` 1))
  (bind _winscreen (`self.WinScreen`))
  (if (`KismetStringLibrary.EqualEqual_StrStr` (`BomberMan3DGameStateBase.result` (`self.GameStateV`)))
    (`Widget.SetVisibility` _winscreen "Hidden")
    (`WidgetBlueprintLibrary.SetInputMode_GameOnly` _returnvalue)
    (set `PlayerController.bShowMouseCursor` false _returnvalue)
    (`WidgetBlueprintLibrary.SetInputMode_GameOnly` _returnvalue_2)
    (set `PlayerController.bShowMouseCursor` false _returnvalue_2)
    (`GameplayStatics.SetGamePaused` false)
    (else
      (`Widget.SetVisibility` _winscreen "Visible")
      (`WidgetBlueprintLibrary.SetInputMode_UIOnlyEx` _returnvalue _winscreen)
      (set `PlayerController.bShowMouseCursor` true _returnvalue)
      (`WidgetBlueprintLibrary.SetInputMode_UIOnlyEx` _returnvalue_2 _winscreen)
      (set `PlayerController.bShowMouseCursor` true _returnvalue_2)
      (`GameplayStatics.SetGamePaused` true))))

(fn `UserConstructionScript`)